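; BP_SnowballFightHUD is the HUD Blueprint for the snowball fight game mode.
; On BeginPlay it creates its HUD widget, adds it to the viewport and sets game-only input for the first player controller.
; SetPowerToHUD and SetAPToHUD forward Power and AP values to that widget for display.
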(event `self.ReceiveBeginPlay`
  (bind _returnvalue (`|CreateWidget` "/Game/SnowballFight/Widget/HUDWidget.HUDWidget_C"))
  (bind _output_get (set `self.HUDWidget` _returnvalue))
  (`UserWidget.AddToViewport` _output_get 0)
  (`WidgetBlueprintLibrary.SetInputMode_GameOnly` (`GameplayStatics.GetPlayerController` 0)))

(fn `SetAPToHUD`
  (params (AP :type "Float (double-precision)"))
  (`/Game/SnowballFight/Widget/HUDWidget.SetAP` (`self.HUDWidget`) AP))

(fn `SetPowerToHUD`
  (params (Power :type "Float (double-precision)"))
  (`/Game/SnowballFight/Widget/HUDWidget.SetPower` (`self.HUDWidget`) Power))

(fn `UserConstructionScript`)