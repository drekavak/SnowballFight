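; BP_LobbyHUD is the lobby HUD for the SnowballFight game mode, showing the lobby widget and switching the player to menu-style input.
; On BeginPlay it creates LobbyHUDWidget, adds it to the viewport, sets UI-only input and shows the mouse cursor.
; UpdatePlayers forwards refresh calls to the widget, retrying itself on a short timer while the widget is not yet valid.
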(event `self.ReceiveBeginPlay`
  (bind _returnvalue (`GameplayStatics.GetPlayerController` 0))
  (bind _returnvalue_2 (`|CreateWidget` "/Game/SnowballFight/Widget/LobbyWidget/LobbyHUDWidget.LobbyHUDWidget_C"))
  (bind _output_get (set `self.LobbyHUDWidget` _returnvalue_2))
  (`UserWidget.AddToViewport` _output_get 0)
  (`WidgetBlueprintLibrary.SetInputMode_UIOnlyEx` _returnvalue null)
  (set `PlayerController.bShowMouseCursor` true _returnvalue))

(fn `UpdatePlayers`
  (bind _lobbyhudwidget (`self.LobbyHUDWidget`))
  (`/Engine/EditorBlueprintResources/StandardMacros.IsValid` _lobbyhudwidget
    (:`Is Valid`
      (`/Game/SnowballFight/Widget/LobbyWidget/LobbyHUDWidget.UpdatePlayers` _lobbyhudwidget))
    (:`Is Not Valid`
      (`KismetSystemLibrary.K2_SetTimer` null "UpdatePlayers" 0.1))))

(fn `UserConstructionScript`)