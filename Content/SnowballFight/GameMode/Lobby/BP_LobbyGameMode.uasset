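; BP_LobbyGameMode is the game mode for the SnowballFight lobby, tracking players as they join and leave.
; PostLogin, HandleStartingNewPlayer and OnLogout each print an on-screen debug message with the display name.
; When a new player starts, it casts the controller to BP_LobbyPlayerController and calls ResStartNewPlayer, printing an error if the cast fails.
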(event `self.K2_PostLogin`
  (params (NewPlayer :type "PlayerController Object Reference"))
  (`KismetSystemLibrary.PrintString` (`KismetStringLibrary.Concat_StrStr` "On Post Login - " (`KismetSystemLibrary.GetDisplayName` NewPlayer)) true true (struct :`G` 0.66 :`B` 1.0 :`A` 1.0) 50.0))

(event `self.HandleStartingNewPlayer`
  (params (NewPlayer :type "PlayerController Object Reference"))
  (`KismetSystemLibrary.PrintString` (`KismetStringLibrary.Concat_StrStr` "Handle Starting New Player - " (`KismetSystemLibrary.GetDisplayName` NewPlayer)))
  (bind _asbp_lobby_player_controller (cast `/Game/SnowballFight/GameMode/Lobby/BP_LobbyPlayerController` NewPlayer)
    (:`then`
      (`/Game/SnowballFight/GameMode/Lobby/BP_LobbyPlayerController.ResStartNewPlayer` _asbp_lobby_player_controller))
    (:`CastFailed`
      (`KismetSystemLibrary.PrintString` "lobbyplayercontroller 캐스트 실패"))))

(event `self.K2_OnLogout`
  (params (ExitingController :type "Controller Object Reference"))
  (`KismetSystemLibrary.PrintString` (`KismetStringLibrary.Concat_StrStr` "OnLogout - " (`KismetSystemLibrary.GetDisplayName` null)) true true (struct :`G` 0.66 :`B` 1.0 :`A` 1.0) 60.0))

(fn `UserConstructionScript`)