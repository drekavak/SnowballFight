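; Game mode for the snowball fight that runs a turn order among the player characters.
; One second after BeginPlay it gathers all SnowballFightCharacters, shuffles them, prints the first three for debugging and starts the first turn.
; CallTurn advances turns through ChooseTurn, which sets IsMyTurn without clearing earlier flags and wraps the index recursively.
; New players trigger ResStartNewPlayer on their controller; the game mode's own Res events are empty.
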(event `self.HandleStartingNewPlayer`
  (params (NewPlayer :type "PlayerController Object Reference"))
  (`parent.HandleStartingNewPlayer` NewPlayer)
  (bind _assnowball_fight_player_controller (cast `/Game/SnowballFight/GameMode/SnowballFightPlayerController` NewPlayer))
  (`/Game/SnowballFight/GameMode/SnowballFightPlayerController.ResStartNewPlayer` _assnowball_fight_player_controller))

(event `self.ReceiveBeginPlay`
  (`KismetSystemLibrary.Delay` 1.0)
  (`self.ReqMakeList`))

(event `ReqMakeList`
  (`self.MakePlayerList`)
  (`self.Do Shuffle`)
  (`self.CheckArray`)
  (`self.ChooseTurn`)
  (`self.ResMakeList`))

(event `ResMakeList`)

(event `Call Turn`
  (`self.ReqChooseTurn`))

(event `ReqChooseTurn`
  (`self.ChooseTurn`)
  (`self.ResChooseTurn`))

(event `ResChooseTurn`)

(fn `CheckArray`
  (`|ExecutionSequence`
    (:`then_0`
      (`KismetSystemLibrary.PrintString` (`KismetStringLibrary.Concat_StrStr` (`KismetSystemLibrary.GetDisplayName` (`|GetArrayItem` (`self.Players`))) " :0번 인덱스") true true (struct :`R` 1.0 :`B` 0.269631 :`A` 1.0) 100.0))
    (:`then_1`
      (`KismetSystemLibrary.PrintString` (`KismetStringLibrary.Concat_StrStr` (`KismetSystemLibrary.GetDisplayName` (`|GetArrayItem` (`self.Players`) 1)) " :1번 인덱스") true true (struct :`R` 1.0 :`B` 0.288289 :`A` 1.0) 100.0))
    (:`then_2`
      (`KismetSystemLibrary.PrintString` (`KismetStringLibrary.Concat_StrStr` (`KismetSystemLibrary.GetDisplayName` (`|GetArrayItem` (`self.Players`) 2)) ": 2번 인덱스") true true (struct :`R` 1.0 :`B` 0.368728 :`A` 1.0) 100.0))))

(fn `ChooseTurn`
  (returns (IsMyTurn :type Boolean))
  (bind _output (`|GetArrayItem` (`self.Players`) (`self.index`)))
  (if (>= (`self.index`) (`self.PlayerNumber`))
    (set `self.index` 0)
    (`self.ChooseTurn`)
    (else
      (`KismetSystemLibrary.PrintString` (`KismetStringLibrary.Concat_StrStr` (`KismetSystemLibrary.GetDisplayName` _output) "의 턴 입니다.") true true (struct :`R` 0.4625 :`G` 0.407707 :`A` 1.0) 100.0)
      (bind _output_get (set `/Game/SnowballFight/GameMode/SnowballFightCharacter.IsMyTurn` true _output))
      (bind _result (`/Engine/EditorBlueprintResources/StandardMacros.IncrementInt` (`self.index`))
        (:`  `
          (set `self.index` _result)
          (return _output_get))))))

(fn `Do Shuffle`
  (`KismetArrayLibrary.Array_Shuffle` (`self.Players`)))

(fn `MakePlayerList`
  (bind _outactors (`GameplayStatics.GetAllActorsOfClass` "/Game/SnowballFight/GameMode/SnowballFightCharacter.SnowballFightCharacter_C"))
  (set `self.Players` _outactors)
  (set `self.PlayerNumber` (`KismetArrayLibrary.Array_Length` _outactors)))

(fn `UserConstructionScript`)