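; Snowball projectile for the snowball fight game that damages the characters it hits.
; On BeginPlay it sets the projectile movement's initial speed from PowerValue and prints it for debugging.
; Its ReqDamageToTarget event takes a hit result and applies fixed damage only if the hit actor is a SnowballFightCharacter.
; The Blueprint binds no collision handling itself; the overlap event is an empty stub.
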(event `self.ReceiveBeginPlay`
  (bind _output_get (set `ProjectileMovementComponent.InitialSpeed` (`self.PowerValue`) (`self.ProjectileMovement`)))
  (`KismetSystemLibrary.PrintString` (`KismetStringLibrary.Conv_DoubleToString` _output_get) true true (struct :`G` 0.66 :`B` 1.0 :`A` 1.0) 30.0))

(event `ReqDamageToTarget`
  (params (HitResult :type "HitResult Structure"))
  (`KismetSystemLibrary.PrintString` "ReqDamageToTarget")
  (`self.DoDamageToTarget` HitResult))

(fn `DoDamageToTarget`
  (params (HitResult :type "HitResult Structure"))
  (bind _assnowball_fight_character (cast `/Game/SnowballFight/GameMode/SnowballFightCharacter` (`.HitActor` (`GameplayStatics.BreakHitResult` HitResult))))
  (`GameplayStatics.ApplyDamage` _assnowball_fight_character 50.0 null self))

(fn `UserConstructionScript`)